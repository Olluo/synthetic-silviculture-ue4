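; BP_BranchModulePrototype1 supplies a fixed branching topology, which by its name serves as a prototype branch module.
; GetGraphDefinition returns a hardcoded GraphDefinition built from directed source-to-destination edges between indexed nodes.
; The edges form a tree: a short trunk chain from node 0 fans out at node 3, and some of those children split again into leaf nodes.
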(fn GetGraphDefinition
  (bind _output_get (Variables|Default|SetGraphDefinition (Utilities|Struct|MakeGraphDefinition (Utilities|Array|MakeArray (Utilities|Struct|MakeGraphEdge 0 1) (Utilities|Struct|MakeGraphEdge 1 2) (Utilities|Struct|MakeGraphEdge 2 3) (Utilities|Struct|MakeGraphEdge 3 4) (Utilities|Struct|MakeGraphEdge 3 5) (Utilities|Struct|MakeGraphEdge 3 6) (Utilities|Struct|MakeGraphEdge 5 7) (Utilities|Struct|MakeGraphEdge 5 8) (Utilities|Struct|MakeGraphEdge 6 9) (Utilities|Struct|MakeGraphEdge 6 10) (Utilities|Struct|MakeGraphEdge 6 11) (Utilities|Struct|MakeGraphEdge 4 12) (Utilities|Struct|MakeGraphEdge 4 13) (Utilities|Struct|MakeGraphEdge 4 14) (Utilities|Struct|MakeGraphEdge 3 15) (Utilities|Struct|MakeGraphEdge 3 16)))))
  (return _output_get))