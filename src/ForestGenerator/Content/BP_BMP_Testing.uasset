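; BP_BMP_Testing is a Blueprint that, by its name, serves as a test asset and supplies a hard-coded graph definition.
; Its only function, GetGraphDefinition, builds the graph from a literal array of source-to-destination edges between integer node indices.
; The edges form a small branching tree of nine nodes rooted at node 0, with branches of uneven depth.
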(fn GetGraphDefinition
  (bind _output_get (Variables|Default|SetGraphDefinition (Utilities|Struct|MakeGraphDefinition (Utilities|Array|MakeArray (Utilities|Struct|MakeGraphEdge 0 1) (Utilities|Struct|MakeGraphEdge 1 2) (Utilities|Struct|MakeGraphEdge 1 3) (Utilities|Struct|MakeGraphEdge 2 4) (Utilities|Struct|MakeGraphEdge 2 5) (Utilities|Struct|MakeGraphEdge 3 6) (Utilities|Struct|MakeGraphEdge 4 7) (Utilities|Struct|MakeGraphEdge 4 8)))))
  (return _output_get))